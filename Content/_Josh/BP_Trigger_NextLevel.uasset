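; Trigger Blueprint that advances the player to the next procedurally generated level.
; When a component tagged Player overlaps its collision component, it increments LevelLength on the GI_LevelData game instance and resets CompletedLevels to zero.
; It prints both values for debugging, showing the completed count plus one, then opens the _Benny_level_procedural level by object reference.
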(event `self.CollisionComponent.OnComponentBeginOverlap`
  (params (OverlappedComponent :type "PrimitiveComponent Object Reference") (OtherActor :type "Actor Object Reference") (OtherComp :type "PrimitiveComponent Object Reference") (OtherBodyIndex :type Integer) (bFromSweep :type Boolean) (SweepResult :type "HitResult Structure (by ref)"))
  (if (`ActorComponent.ComponentHasTag` OtherComp "Player")
    (bind _asgi_level_data (cast `/Game/_Josh/GI_LevelData` (`GameplayStatics.GetGameInstance`)))
    (bind _output_get (set `/Game/_Josh/GI_LevelData.LevelLength` (+ (`/Game/_Josh/GI_LevelData.LevelLength` _asgi_level_data) 1) _asgi_level_data))
    (`KismetSystemLibrary.PrintString` (`KismetStringLibrary.Concat_StrStr` "New LevelLength:" (`KismetStringLibrary.Conv_IntToString` _output_get)))
    (set `/Game/_Josh/GI_LevelData.CompletedLevels` 0 _asgi_level_data)
    (`KismetSystemLibrary.PrintString` (`KismetStringLibrary.Concat_StrStr` "Completed Levels:" (`KismetStringLibrary.Conv_IntToString` (+ (`/Game/_Josh/GI_LevelData.CompletedLevels` _asgi_level_data) 1))))
    (`GameplayStatics.OpenLevelBySoftObjectPtr` "/Game/Maps/_Benny_level_procedural._Benny_level_procedural")))

(fn `UserConstructionScript`)