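; AI spawn point placeholder that replaces itself with a random turret, grunt or Roomba on BeginPlay.
; A three-way random roll picks the class, which spawns using the scene root's relative transform.
; The new actor attaches to the spawn point's parent actor with keep-relative rules, so that transform becomes its offset within the parent.
; The spawn point then destroys itself.
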(event `self.ReceiveBeginPlay`
  (bind _returnvalue (`SceneComponent.GetRelativeTransform` (`self.DefaultSceneRoot`)))
  (switch `int` (`KismetMathLibrary.RandomInteger` 3)
    (:`0`
      (bind _returnvalue_2 (`|SpawnActorFromClass` "/Game/BPs/EnemyStuff/BP_Turret.BP_Turret_C" _returnvalue "Undefined" "OverrideRootScale" null null))
      (bind _output_get (set `self.spawnedActor` _returnvalue_2)))
    (:`1`
      (bind _returnvalue_3 (`|SpawnActorFromClass` "/Game/BPs/EnemyStuff/BP_Grunt.BP_Grunt_C" _returnvalue "Undefined" "OverrideRootScale" null null))
      (bind _output_get_2 (set `self.spawnedActor` _returnvalue_3)))
    (:`2`
      (bind _returnvalue_4 (`|SpawnActorFromClass` "/Game/BPs/EnemyStuff/BP_Roomba.BP_Roomba_C" _returnvalue "Undefined" "OverrideRootScale" null null))
      (bind _output_get_3 (set `self.spawnedActor` _returnvalue_4))))
  (`self.K2_AttachToActor` _output_get_2 (`self.GetAttachParentActor`) "None" "KeepRelative" "KeepRelative" "KeepRelative" false)
  (`self.K2_AttachToActor` _output_get_3 (`self.GetAttachParentActor`) "None" "KeepRelative" "KeepRelative" "KeepRelative" false)
  (`self.K2_AttachToActor` _output_get (`self.GetAttachParentActor`) "None" "KeepRelative" "KeepRelative" "KeepRelative" false)
  (`self.K2_DestroyActor`))

(fn `UserConstructionScript`)