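; Rocket-launcher grunt enemy that turns alert on first sighting a pawn, then faces and tracks BennyCharacter on later sightings.
; Pawn sensing eases an aim Distance toward the player's range, which Tick uses as launch speed to predict an arc from the muzzle and place a decal at its end.
; Tick also animates the launcher coils.
; A delay toggles SpawnProjectile, but its branch is disconnected, so no rocket spawns here.
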(event `self.ReceiveTick`
  (params (DeltaSeconds :type "Float (single-precision)"))
  (bind (_returnvalue_location _returnvalue_rotation) (`KismetMathLibrary.BreakTransform` (`SceneComponent.GetSocketTransform` (`self.RocketLauncher`) "mouth" "RTS_World")))
  (`SceneComponent.K2_SetRelativeRotation` (`self.RocketLauncher_CharginCoils`) (`KismetMathLibrary.MakeRotator` 0.0 (`GameplayStatics.GetTimeSeconds`)) false false)
  (`/Engine/EditorBlueprintResources/StandardMacros.Gate` false
    (:`Exit`
      (bind (_outhit _outpathpositions _outlasttracedestination) (`GameplayStatics.Blueprint_PredictProjectilePath_ByObjectType` :`StartPos` _returnvalue_location :`LaunchVelocity` (* (`KismetMathLibrary.GetForwardVector` _returnvalue_rotation) (`self.distance`)) :`ObjectTypes` (`|MakeArray` "ObjectTypeQuery1" :!type "EObjectTypeQuery Enum") :`DrawDebugType` "ForDuration" :`SimFrequency` 10.0))
      (`SceneComponent.K2_SetWorldLocation` (`self.Decal`) _outlasttracedestination false false))))

(event `self.PawnSensing.OnSeePawn`
  (params (Pawn :type "Pawn Object Reference"))
  (if (`self.alerted`)
    (bind _as_benny_character (cast `/Game/_Benny/_BennyCharacter` Pawn))
    (`|ExecutionSequence`
      (:`then_0`
        ;[1 1 1] Rotate
        (`self.K2_SetActorRotation` (`KismetMathLibrary.FindLookAtRotation` (`self.K2_GetActorLocation`) (`self.K2_GetActorLocation` _as_benny_character))))
      (:`then_1`
        ;[1 1 1] Spawn Rocket
        (set `self.distance` (`KismetMathLibrary.FInterpTo` (`self.distance`) (`KismetMathLibrary.Vector_Distance` (`self.K2_GetActorLocation`) (`self.K2_GetActorLocation` _as_benny_character)) 0.005 (`self.trackSpeed`))))
      (:`then_2`
        ;[1 1 1] Delay between shot
        (set `self.spawnProjectile` false)
        (`KismetSystemLibrary.Delay` (`self.shootDelay`))
        (set `self.spawnProjectile` true)))
    (else
      (set `self.alerted` true)
      (set `self.idling` false))))

(fn `UserConstructionScript`)