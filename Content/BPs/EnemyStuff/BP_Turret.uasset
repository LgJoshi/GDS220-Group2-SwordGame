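; Enemy laser turret that spots the player's BennyCharacter through PawnSensing and attacks with a telegraphed beam.
; Once alerted, it yaws toward the player while charging, then locks aim, widens the beam, fires and cools down using chained delays.
; Tick updates the beam endpoints and, on a 0.2-second Delay, runs a box trace that damages the player or cover during firing.
; A Dead flag disables sensing and Tick logic.
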(event `self.ReceiveBeginPlay`
  (set `self.DeathSound` "/Game/Audio/sfx/Turret_Death.Turret_Death"))

(event `self.PawnSensing.OnSeePawn`
  (params (Pawn :type "Pawn Object Reference"))
  (bind __josh_parti_laser (`self._Josh_parti_laser`))
  (if (`self.dead`)
    _
    (elif (`self.alerted`)
      (bind _as_benny_character (cast `/Game/_Benny/_BennyCharacter` Pawn))
      (`/Engine/EditorBlueprintResources/StandardMacros.IsValid` _as_benny_character
        (:`Is Valid`
          (`|ExecutionSequence`
            (:`then_0`
              ;[1 1 1] Rotate
              (if (`self.charging`)
                (bind (_returnvalue_roll _returnvalue_pitch _returnvalue_yaw) (`KismetMathLibrary.BreakRotator` (`KismetMathLibrary.RInterpTo_Constant` (`SceneComponent.K2_GetComponentRotation` (`self.turret_chassis_Chasi`)) (`KismetMathLibrary.FindLookAtRotation` (`SceneComponent.K2_GetComponentLocation` (`self.Turret_Base`)) (`self.K2_GetActorLocation` _as_benny_character)) 1.0 (`self.rotateSpeed`))))
                (`SceneComponent.K2_SetWorldRotation` (`self.turret_chassis_Chasi`) (`KismetMathLibrary.MakeRotator` 0.0 0.0 _returnvalue_yaw) false false)))
            (:`then_1`
              ;[1 1 1] Rotating
              (if (not (`self.shooting`))
                (set `self.charging` true)
                (set `self.shooting` true)
                (`KismetSystemLibrary.Delay` (`self.chargeTime`))
                ;[1 1 1] Start Charging
                (`FXSystemComponent.SetVectorParameter` __josh_parti_laser "size" (5.0 1.0 1.0))
                (set `self.charging` false)
                (`GameplayStatics.PlaySound2D` "/Game/Audio/sfx/Turret_Charge.Turret_Charge" 1.0 1.0 0.0 null null)
                (`KismetSystemLibrary.Delay` (`self.shootDelay`))
                ;[1 1 1] Firing
                (`FXSystemComponent.SetVectorParameter` __josh_parti_laser "size" (20.0 1.0 1.0))
                (`GameplayStatics.PlaySound2D` "/Game/Audio/sfx/Turret_Fire.Turret_Fire" 1.0 1.0 0.0 null null)
                (set `self.castingBox` true)
                (`KismetSystemLibrary.Delay` (`self.cooldown`))
                (`GameplayStatics.PlaySound2D` "/Game/Audio/sfx/Turret_Stop_take_2.Turret_Stop_take_2" 0.4 0.5 0.0 null null)
                (set `self.castingBox` false)
                (`FXSystemComponent.SetVectorParameter` (`self._Josh_parti_laser`) "size" (1.0 1.0 1.0))
                (set `self.alerted` false)
                (set `self.shooting` false)
                (goto _label :!via `Reset`))))))
      (else
        (`/Engine/EditorBlueprintResources/StandardMacros.DoOnce` false :!label _label
          (:`Completed`
            (set `self.alerted` true)))))))

(event `self.ReceiveTick`
  (params (DeltaSeconds :type "Float (single-precision)"))
  (bind __josh_parti_laser (`self._Josh_parti_laser`))
  (bind _turret_gun_turret (`self.turret_gun_Turret`))
  (bind _returnvalue (`SceneComponent.K2_GetComponentLocation` (`self.Firing Point`)))
  (bind _returnvalue_2 (`SceneComponent.K2_GetComponentLocation` _turret_gun_turret))
  (if (not (`self.dead`))
    (`|ExecutionSequence`
      (:`then_0`
        ;[1 1 1] Tick Laser
        (`KismetSystemLibrary.Delay` 0.2)
        (`self.Boxcast Damage`))
      (:`then_1`
        ;[1 1 1] Check if Alerted
        (if (`self.alerted`)
          (`ParticleSystemComponent.SetBeamSourcePoint` __josh_parti_laser 0 _returnvalue 0)
          ;[1 1 1] Laser LineTrace Particle
          (bind _outhit (`KismetSystemLibrary.LineTraceSingleForObjects` :`Start` _returnvalue_2 :`End` (+ _returnvalue_2 (* (`SceneComponent.GetForwardVector` _turret_gun_turret) 10000)) :`ObjectTypes` (`|MakeArray` "ObjectTypeQuery1" "ObjectTypeQuery10" :!type "EObjectTypeQuery Enum") :`DrawDebugType` "ForOneFrame"))
          (`ParticleSystemComponent.SetBeamEndPoint` (`self._Josh_parti_laser`) 0 (`.TraceEnd` (`GameplayStatics.BreakHitResult` _outhit)))
          (else
            (`ParticleSystemComponent.SetBeamEndPoint` __josh_parti_laser 0 _returnvalue)))))))

(fn `Boxcast Damage`
  (bind _turret_gun_turret (`self.turret_gun_Turret`))
  (bind _returnvalue (`SceneComponent.K2_GetComponentLocation` (`self.Firing Point`)))
  ;[1 1 1] If hit player: do once. Reset after 0.5s.
  (if (`self.castingBox`)
    (bind _outhit (`KismetSystemLibrary.BoxTraceSingleForObjects` _returnvalue (+ _returnvalue (* (`SceneComponent.GetForwardVector` _turret_gun_turret) 10000)) (0.0 40.0 40.0) (`SceneComponent.K2_GetComponentRotation` _turret_gun_turret) (`|MakeArray` "ObjectTypeQuery3" "ObjectTypeQuery1" "ObjectTypeQuery6" :!type "EObjectTypeQuery Enum")))
    (bind (_bblockinghit _binitialoverlap _time _distance _location _impactpoint _normal _impactnormal _physmat _hitactor) (`GameplayStatics.BreakHitResult` _outhit))
    (bind _as_benny_character (cast `/Game/_Benny/_BennyCharacter` _hitactor)
      (:`then`
        (`/Engine/EditorBlueprintResources/StandardMacros.IsValid` _hitactor
          (:`Is Valid`
            (`/Game/_Benny/_BennyCharacter.ReceiveDamage` _as_benny_character))))
      (:`CastFailed`
        (bind _as_josh_bp_cover (cast `/Game/BPs/Props/_Josh_BP_Cover` _hitactor))
        (`/Game/BPs/Props/_Josh_BP_Cover.Take Damage` _as_josh_bp_cover)))))

(fn `UserConstructionScript`)