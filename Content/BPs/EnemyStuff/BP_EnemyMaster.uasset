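; BP_EnemyMaster is an enemy Blueprint whose only logic handles death.
; DeathFunction prints a death message, then casts its attach parent actor to BP_RoomController and calls CheckKeyCondition.
; It then sets the DeathANIM flag on the mesh's Anim_master_enemy instance.
; The casts are chained, so an enemy not attached to a room controller never sets the death animation flag.
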(fn `DeathFunction`
  (`KismetSystemLibrary.PrintString` (`KismetStringLibrary.Concat_StrStr` (`KismetSystemLibrary.GetObjectName` self) ": I died"))
  (bind _asbp_room_controller (cast `/Game/BPs/BP_RoomController` (`self.GetAttachParentActor`)))
  (`/Game/BPs/BP_RoomController.CheckKeyCondition` _asbp_room_controller)
  (bind _asanim_master_enemy (cast `/Game/Models/Guard/Anim_master_enemy` (`SkeletalMeshComponent.GetAnimInstance` (`self.Mesh`))))
  (set `/Game/Models/Guard/Anim_master_enemy.DeathANIM` true _asanim_master_enemy))

(fn `UserConstructionScript`)