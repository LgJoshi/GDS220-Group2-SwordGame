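; BP_Door is a lockable door prop that sinks down when the Benny character enters its trigger box and returns when they leave.
; Tick continuously eases the door's relative location toward the open or closed position based on the Opening flag.
; Overlaps change that flag and play sounds at world origin only while Unlocked is set.
; The Unlock function sets that state and switches the frame to an emissive material, which BeginPlay also applies if already unlocked.
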(event `self.ReceiveBeginPlay`
  (if (`self.unlocked`)
    (`PrimitiveComponent.SetMaterial` (`self.door_frame`) 1 "/Game/Models/Turret/Emit2.Emit2")))

(event `self.ReceiveTick`
  (params (DeltaSeconds :type "Float (single-precision)"))
  (bind _door (`self.door`))
  (if (`self.opening`)
    (`SceneComponent.K2_SetRelativeLocation` _door (`KismetMathLibrary.VLerp` (`SceneComponent.RelativeLocation` _door) (0.0 0.0 -910.0) 0.05) false false)
    (else
      (`SceneComponent.K2_SetRelativeLocation` _door (`KismetMathLibrary.VLerp` (`SceneComponent.RelativeLocation` _door) (0.0 0.0 0.0) 0.05) false false))))

(event `self.Box.OnComponentBeginOverlap`
  (params (OverlappedComponent :type "PrimitiveComponent Object Reference") (OtherActor :type "Actor Object Reference") (OtherComp :type "PrimitiveComponent Object Reference") (OtherBodyIndex :type Integer) (bFromSweep :type Boolean) (SweepResult :type "HitResult Structure (by ref)"))
  (`KismetSystemLibrary.PrintString` (`KismetSystemLibrary.GetDisplayName` OtherActor))
  (if (== (`GameplayStatics.GetObjectClass` OtherActor) "/Game/_Benny/_BennyCharacter._BennyCharacter_C")
    (if (`self.unlocked`)
      (set `self.opening` true)
      (`GameplayStatics.PlaySoundAtLocation` "/Game/Audio/sfx/Door_Open.Door_Open" (0.0 0.0 0.0) (struct) 1.0 1.0 0.0 null null null))))

(event `self.Box.OnComponentEndOverlap`
  (params (OverlappedComponent :type "PrimitiveComponent Object Reference") (OtherActor :type "Actor Object Reference") (OtherComp :type "PrimitiveComponent Object Reference") (OtherBodyIndex :type Integer))
  (if (== (`GameplayStatics.GetObjectClass` OtherActor) "/Game/_Benny/_BennyCharacter._BennyCharacter_C")
    (if (`self.unlocked`)
      (set `self.opening` false)
      (`GameplayStatics.PlaySoundAtLocation` "/Game/Audio/sfx/Door_Close.Door_Close" (0.0 0.0 0.0) (struct) 1.0 1.0 0.0 null null null))))

(fn `Unlock`
  (set `self.unlocked` true)
  (`KismetSystemLibrary.PrintString` "unlocked")
  (`PrimitiveComponent.SetMaterial` (`self.door_frame`) 1 "/Game/Models/Turret/Emit2.Emit2"))

(fn `UserConstructionScript`)