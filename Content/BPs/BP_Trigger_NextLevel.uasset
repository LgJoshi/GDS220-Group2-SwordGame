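; Trigger Blueprint that advances the game to a new, longer run of the procedural level when the player overlaps it.
; An overlap by a component tagged "Player" increments LevelLength on GI_myGameInstance and resets CompletedLevels to zero, printing debug messages for both.
; It then opens the mainprocedural level, with the game instance carrying the updated values across the load.
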(event `self.CollisionComponent.OnComponentBeginOverlap`
  (params (OverlappedComponent :type "PrimitiveComponent Object Reference") (OtherActor :type "Actor Object Reference") (OtherComp :type "PrimitiveComponent Object Reference") (OtherBodyIndex :type Integer) (bFromSweep :type Boolean) (SweepResult :type "HitResult Structure (by ref)"))
  (if (`ActorComponent.ComponentHasTag` OtherComp "Player")
    (bind _asgi_my_game_instance (cast `/Game/BPs/GI_myGameInstance` (`GameplayStatics.GetGameInstance`)))
    (bind _output_get (set `/Game/BPs/GI_myGameInstance.LevelLength` (+ (`/Game/BPs/GI_myGameInstance.LevelLength` _asgi_my_game_instance) 1) _asgi_my_game_instance))
    (`KismetSystemLibrary.PrintString` (`KismetStringLibrary.Concat_StrStr` "New LevelLength:" (`KismetStringLibrary.Conv_IntToString` _output_get)))
    (set `/Game/BPs/GI_myGameInstance.CompletedLevels` 0 _asgi_my_game_instance)
    (`KismetSystemLibrary.PrintString` (`KismetStringLibrary.Concat_StrStr` "Completed Levels:" (`KismetStringLibrary.Conv_IntToString` (+ (`/Game/BPs/GI_myGameInstance.CompletedLevels` _asgi_my_game_instance) 1))))
    (`GameplayStatics.OpenLevelBySoftObjectPtr` "/Game/Maps/level_mainprocedural.level_mainprocedural")))

(fn `UserConstructionScript`)