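; Room controller that unlocks its door once a randomly chosen number of key checks is reached.
; On BeginPlay it takes the last attached actor as the door and rolls the target from the attached actor count.
; CheckKeyCondition increments a counter and, at the target, calls UnlockDoor through a DoOnce.
; Pressing 1 unlocks the door directly, and print strings trace the setup and checks.
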(event `Key|One`
  (params (Key :type "Key Structure"))
  (:`Pressed`
    (`KismetSystemLibrary.PrintString` "press 1")
    (bind _asbp_door (cast `/Game/BPs/BP_Door` (`self.thisRoomDoor`)))
    (`/Game/BPs/BP_Door.Unlock` _asbp_door)))

(event `self.ReceiveBeginPlay`
  (bind _outactors (`self.GetAttachedActors` true))
  (bind _returnvalue (`KismetArrayLibrary.Array_Length` _outactors))
  (bind _output (`|GetArrayItem` _outactors (- _returnvalue 1)))
  (`KismetSystemLibrary.PrintString` (`KismetSystemLibrary.GetDisplayName` _output))
  (set `self.thisRoomDoor` _output)
  (bind _output_get (set `self.targetKey` (+ (`KismetMathLibrary.RandomInteger` (- _returnvalue 2)) 1)))
  (`KismetSystemLibrary.PrintString` (`KismetStringLibrary.Concat_StrStr` "Target Key: " (`KismetStringLibrary.Conv_IntToString` _output_get))))

(fn `CheckKeyCondition`
  (`KismetSystemLibrary.PrintString` "checking key")
  (set `self.currentKey` (+ (`self.currentKey`) 1))
  (if (>= (`self.currentKey`) (`self.targetKey`))
    (`/Engine/EditorBlueprintResources/StandardMacros.DoOnce` false
      (:`Completed`
        (`self.UnlockDoor`)))))

(fn `UnlockDoor`
  (bind _asbp_door (cast `/Game/BPs/BP_Door` (`self.thisRoomDoor`)))
  (`/Game/BPs/BP_Door.Unlock` _asbp_door))

(fn `UserConstructionScript`)