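; BP_Door is a lockable sliding door that lowers while the Benny character stands in its trigger box, once unlocked.
; Box overlaps set the Opening flag, and Tick eases the door between lowered and raised positions with a fixed-alpha, frame-rate-dependent lerp.
; Unlock sets the Unlocked flag and swaps the door to the Emit2 material.
; OpenDoor snaps an unlocked door down, though Tick keeps easing it toward the flag's position.
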(event `self.ReceiveTick`
  (params (DeltaSeconds :type "Float (single-precision)"))
  (bind _door (`self.door`))
  (if (`self.opening`)
    (`SceneComponent.K2_SetRelativeLocation` _door (`KismetMathLibrary.VLerp` (`SceneComponent.RelativeLocation` _door) (0.0 0.0 -270.0) 0.1) false false)
    (else
      (`SceneComponent.K2_SetRelativeLocation` _door (`KismetMathLibrary.VLerp` (`SceneComponent.RelativeLocation` _door) (0.0 0.0 270.0) 0.1) false false))))

(event `self.Box.OnComponentBeginOverlap`
  (params (OverlappedComponent :type "PrimitiveComponent Object Reference") (OtherActor :type "Actor Object Reference") (OtherComp :type "PrimitiveComponent Object Reference") (OtherBodyIndex :type Integer) (bFromSweep :type Boolean) (SweepResult :type "HitResult Structure (by ref)"))
  (`KismetSystemLibrary.PrintString` (`KismetSystemLibrary.GetDisplayName` OtherActor))
  (if (== (`GameplayStatics.GetObjectClass` OtherActor) "/Game/_Benny/_BennyCharacter._BennyCharacter_C")
    (if (`self.unlocked`)
      (set `self.opening` true))))

(event `self.Box.OnComponentEndOverlap`
  (params (OverlappedComponent :type "PrimitiveComponent Object Reference") (OtherActor :type "Actor Object Reference") (OtherComp :type "PrimitiveComponent Object Reference") (OtherBodyIndex :type Integer))
  (if (== (`GameplayStatics.GetObjectClass` OtherActor) "/Game/_Benny/_BennyCharacter._BennyCharacter_C")
    (set `self.opening` false)))

(fn `Open Door`
  (`KismetSystemLibrary.PrintString` "openig")
  (if (`self.unlocked`)
    (`SceneComponent.K2_SetRelativeLocation` (`self.door`) (0.0 0.0 -270.0) false false)
    (else
      (`KismetSystemLibrary.PrintString` "not unlocked"))))

(fn `Unlock`
  (set `self.unlocked` true)
  (`KismetSystemLibrary.PrintString` "unlocked")
  (`PrimitiveComponent.SetMaterial` (`self.door`) 0 "/Game/Models/Turret/Emit2.Emit2"))

(fn `UserConstructionScript`)